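; TwinBP is an AI actor Blueprint that handles its own death and supplies random navigation points.
; OnDeath activates a particle system, plays an explosion sound at the actor's location and starts a short timer that destroys the actor, leaving a brief window for the effect.
; RandomPoint returns a random reachable navmesh location within a very large radius around the actor; no caller appears in this Blueprint.
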(event Custom|CustomEvent_0
  (Actor|DestroyActor))

(event EventBeginPlay)

(event Collision|EventActorBeginOverlap
  (params (OtherActor :type Actor%20Object%20Reference)))

(event EventTick
  (params (DeltaSeconds :type Float%20%28single-precision%29)))

(event EventOnDeath
  (Components|Activation|Activate (Variables|Default|GetParticleSystem) false)
  (Audio|PlaySoundatLocation "/Game/StarterContent/Audio/Explosion01.Explosion01" (Transformation|GetActorLocation) "0, 0, 0" 1.0 1.0 0.0 0 0 0)
  (Utilities|Time|SetTimerbyEvent (delegate Custom|CustomEvent_0) 0.6))

(fn ConstructionScript)

(fn RandomPoint
  (return (.RandomLocation (AI|Navigation|GetRandomReachablePointinRadius (Transformation|GetActorLocation) 1e+05 0 0))))